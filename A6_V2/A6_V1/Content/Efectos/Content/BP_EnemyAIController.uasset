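; AI controller for enemies that starts the enemy blackboard and behavior tree on BeginPlay.
; AI Perception updates react only to the top-down player character, writing it and its last known location to the blackboard when sensed.
; On losing perception, a retriggerable five-second delay runs before clearing the player key, leaving the last known location in place.
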(event OnTargetPerceptionUpdated(AIPerception)
  (params (Actor :type Actor%20Object%20Reference) (Stimulus :type AI%20Stimulus%20Structure))
  (bind _returnvalue (AI|GetBlackboard 0))
  (bind _asbp_top_down_character (Utilities|Casting|CastToBP_TopDownCharacter Actor))
  (if (.bSuccessfullySensed (Utilities|Struct|BreakAIStimulus Stimulus))
    (AI|Components|Blackboard|SetValueasObject _returnvalue (Utilities|Name|MakeLiteralName "PlayerActor") _asbp_top_down_character)
    (AI|Components|Blackboard|SetValueasVector _returnvalue (Utilities|Name|MakeLiteralName "LastKnownLocation") (Transformation|GetActorLocation _asbp_top_down_character))
    (else
      (Utilities|FlowControl|RetriggerableDelay 5.0)
      (AI|Components|Blackboard|ClearValue (AI|GetBlackboard 0) (Utilities|Name|MakeLiteralName "PlayerActor")))))

(event EventBeginPlay
  (Class|AIController|UseBlackboard "/Game/BB_Enemy.BB_Enemy")
  (AI|RunBehaviorTree "/Game/BT_Enemy.BT_Enemy"))

(event EventTick
  (params (DeltaSeconds :type Float%20%28single-precision%29)))

(fn ConstructionScript)